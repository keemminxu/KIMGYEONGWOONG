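; BP_TmpPlayer is a temporary player Blueprint that shows an HP bar and drains a CurPosion value over time.
; On BeginPlay it creates the HUD_HP_Bar widget, stores the reference and adds it to the viewport.
; Tick accumulates delta time and, each time it reaches DescresingTime, lowers CurPosion by a fixed step and resets the timer.
; The drain has no clamp, and this graph never passes the value to the widget.
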(event EventBeginPlay
  (bind _returnvalue (UserInterface|CreateWidget "/Game/GYEONG/Blueprints/HUD_HP_Bar.HUD_HP_Bar_C"))
  (bind _output_get (Variables|Default|SetHP_reference _returnvalue))
  (UserInterface|Viewport|AddtoViewport _output_get 0))

(event Collision|EventActorBeginOverlap
  (params (OtherActor :type Actor%20Object%20Reference)))

(event EventTick
  (params (DeltaSeconds :type Float%20%28single-precision%29))
  (bind _output_get (Variables|Default|SetcurrentTime (+ DeltaSeconds (Variables|Default|GetcurrentTime))))
  (if (>= _output_get (Variables|Default|GetdescresingTime))
    (Variables|Default|SetcurPosion (- (Variables|Default|GetcurPosion) 1e+01))
    (Variables|Default|SetcurrentTime 0.0)))

(fn ConstructionScript)