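; BP_Shield is a short-lived moving shield actor that destroys itself through a lifespan set at BeginPlay.
; Each Tick it moves itself along its Direction variable, scaled by Speed and delta time, without sweeping for collisions.
; An unconnected node would aim Direction from the shield toward the Playerlocation actor, but it never runs, so this graph never updates Direction.
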(event EventBeginPlay
  (Actor|SetLifeSpan 5.0))

(event Collision|EventActorBeginOverlap
  (params (OtherActor :type Actor%20Object%20Reference)))

(event EventTick
  (params (DeltaSeconds :type Float%20%28single-precision%29))
  (Transformation|SetActorLocation (+ (* (* (Variables|Default|GetDirection) (Variables|Default|Getspeed)) DeltaSeconds) (Transformation|GetActorLocation)) false false))

(fn ConstructionScript)