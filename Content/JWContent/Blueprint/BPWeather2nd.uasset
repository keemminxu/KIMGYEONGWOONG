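; BPWeather2nd is a weather Blueprint that toggles the sky between a blue, light-cloud look and a dark gray one on the C key.
; A FlipFlop plays or reverses a timeline that lerps SkyRef's sky material colors and a scalar, though some parameter names are None.
; The LightRef color is also set, but its lerp alpha is fixed at zero, so it stays constant.
; The BeginPlay timer targets an empty SetWeatherTime event with zero time.
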(event Custom|SetWeatherTime)

(event EventBeginPlay
  (Utilities|Time|SetTimerbyEvent (delegate Custom|SetWeatherTime) 0.0))

(event Collision|EventActorBeginOverlap
  (params (OtherActor :type Actor%20Object%20Reference)))

(event EventTick
  (params (DeltaSeconds :type Float%20%28single-precision%29)))

(event Input|KeyboardEvents|C
  (params (Key :type Key%20Structure :default "None"))
  (bind _skyref (Variables|Default|GetSkyRef))
  (bind _sky_material (Variables|/Engine/EngineSky/BP_Sky_Sphere.BP_Sky_Sphere_C|GetSky%20material _skyref))
  (:Pressed
    (if (Utilities|IsValid (Variables|Default|GetSkyRef))
      (Utilities|FlowControl|FlipFlop
        (:A
          (bind _newtrack_0 (Timeline|Timeline_1 Play)
            (:Update
              (Rendering|Material|SetVectorParameterValue _sky_material "None" (Math|Color|Lerp(LinearColor) "(R=0.012573,G=0.046246,B=0.317708,A=1.000000)" "(R=0.135417,G=0.135417,B=0.135417,A=1.000000)" _newtrack_0) :!class /Script/Engine.MaterialInstanceDynamic)
              (Rendering|Material|SetVectorParameterValue _sky_material "Horizon Color" (Math|Color|Lerp(LinearColor) "(R=0.036070,G=0.132674,B=0.911458,A=1.000000)" "(R=0.135417,G=0.135417,B=0.135417,A=1.000000)" _newtrack_0) :!class /Script/Engine.MaterialInstanceDynamic)
              (Rendering|Material|SetVectorParameterValue _sky_material "Cloud Color" (Math|Color|Lerp(LinearColor) "(R=0.911458,G=0.872312,B=0.881470,A=1.000000)" "(R=0.036458,G=0.036458,B=0.036458,A=1.000000)" _newtrack_0) :!class /Script/Engine.MaterialInstanceDynamic)
              (Rendering|Material|SetScalarParameterValue _sky_material "None" (Math|Float|Lerp 1.2 5.0 _newtrack_0) :!class /Script/Engine.MaterialInstanceDynamic)
              (Rendering|Components|Light|SetLightColor (Variables|/Script/Engine.Light|GetLightComponent (Variables|Default|GetLightRef)) (Math|Color|Lerp(LinearColor) "(R=0.911458,G=0.872312,B=0.881470,A=1.000000)" "(R=0.000000,G=0.000000,B=0.000000,A=1.000000)" 0.0) true))))
        (:B
          (Timeline|Timeline_1 Reverse))))))

(fn ConstructionScript)