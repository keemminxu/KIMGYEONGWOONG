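; Player character Blueprint for melee sword combat, handling camera-relative movement, attacks, rolling and damage.
; Attack plays one of two random montages, Shift selects the special pair, and IsAttack blocks movement and new actions during attacks and rolls.
; Collision events toggle the sword Box, whose hits apply fixed damage.
; BeginPlay sets up BP_Condition status bars; incoming damage lowers HP, updates its bar and spawns a BP_Damage overlay.
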(event OnComponentHit(Box)
  (params (HitComponent :type Primitive%20Component%20Object%20Reference) (OtherActor :type Actor%20Object%20Reference) (OtherComp :type Primitive%20Component%20Object%20Reference) (NormalImpulse :type Vector :default "0, 0, 0") (Hit :type Hit%20Result%20Structure%20%28by%20ref%29))
  ;[1 1 1] 검으로 공격받은 물체 데미지 입력
  (Game|Damage|ApplyDamage OtherActor 1e+01 0 0))

(event Custom|OnAnimEnd_Attack
  ;[1 1 1] 공격 완료
  (Variables|Default|SetisAttack false))

(event Custom|OnCollisionStart_Attack
  ;[1 1 1] 칼 충돌 설정(공격시에만 충돌 처리)
  (Collision|SetCollisionEnabled (Variables|Default|GetBox) "QueryAndPhysics"))

(event Custom|OnCollisionEnd_Attack
  ;[1 1 1] 칼 충돌 설정(공격시에만 충돌 처리)
  (Collision|SetCollisionEnabled (Variables|Default|GetBox) "NoCollision"))

(event EventBeginPlay
  ;[1 1 1] 상태바 위젯 호출
  (bind _returnvalue (UserInterface|CreateWidget "/Game/JWContent/Blueprint/BP_Condition.BP_Condition_C" (Game|GetPlayerController 0)))
  (bind _output_get (Variables|Default|SetCondition _returnvalue))
  (UserInterface|Viewport|AddtoViewport _output_get 0)
  ;[1 1 1] 에너지바 호출
  (bind _asbp_condition (Utilities|Casting|CastToBP_Condition (UserInterface|GetUserWidgetObject (Variables|Default|Getplayerwidget))))
  (bind _output_get_2 (Variables|Default|SetAs%20BP%20Condition _asbp_condition))
  (Variables|/Game/JWContent/Blueprint/BP_Condition.BP_Condition_C|SetHPBarInput _output_get_2 1.0)
  (bind _asbp_condition_2 (Utilities|Casting|CastToBP_Condition (UserInterface|GetUserWidgetObject (Variables|Default|Getplayerwidget))))
  (bind _output_get_3 (Variables|Default|SetAs%20BP%20Condition_0 _asbp_condition_2))
  (Variables|/Game/JWContent/Blueprint/BP_Condition.BP_Condition_C|SetMPBarInput _output_get_3 1.0)
  (bind _asbp_condition_3 (Utilities|Casting|CastToBP_Condition (UserInterface|GetUserWidgetObject (Variables|Default|Getplayerwidget))))
  (bind _output_get_4 (Variables|Default|SetAs%20BP%20Condition_1 _asbp_condition_3))
  (Variables|/Game/JWContent/Blueprint/BP_Condition.BP_Condition_C|SetSTABarInput _output_get_4 1.0))

(event Collision|EventActorBeginOverlap
  (params (OtherActor :type Actor%20Object%20Reference)))

(event EventTick
  (params (DeltaSeconds :type Float%20%28single-precision%29)))

(event Game|Damage|EventAnyDamage
  (params (Damage :type Float%20%28single-precision%29) (DamageType :type Damage%20Type%20Object%20Reference) (InstigatedBy :type Controller%20Object%20Reference) (DamageCauser :type Actor%20Object%20Reference))
  ;[1 1 1] 데미지 입력
  (CallFunction|DamageUIEvent)
  (Variables|Default|SetHP (- (Variables|Default|GetHP) Damage))
  ;[1 1 1] 에너지 잔량 입력
  (Variables|/Game/JWContent/Blueprint/BP_Condition.BP_Condition_C|SetHPBarInput (Variables|Default|GetAs%20BP%20Condition) (/ (Variables|Default|GetHP) (Variables|Default|GetHPNorm))))

(event Input|ActionEvents|InputActionAttack
  (params (Key :type Key%20Structure :default "None"))
  ;[1 1 1] 공격 모션 기본 속공 랜덤
  (:Pressed
    (if (not (Variables|Default|GetisAttack))
      ;[1 1 1] 특수 공격 Shift + Mouse Left
      (if (Variables|Default|GetSAttack)
        (if (<= (Math|Random|RandomIntegerinRange 1 2) 1)
          (Animation|PlayAnimMontage "/Game/JWContent/Anim/360_Jump_Attack_Montage.360_Jump_Attack_Montage" 1.0 "None")
          (Variables|Default|SetisAttack true)
          (else
            (Animation|PlayAnimMontage "/Game/JWContent/Anim/TwoAttack_Montage.TwoAttack_Montage" 1.0 "None")
            (Variables|Default|SetisAttack true)))
        (elif (<= (Math|Random|RandomIntegerinRange 1 2) 1)
          (Animation|PlayAnimMontage "/Game/JWContent/Anim/Attack1_Montage.Attack1_Montage" 1.0 "None")
          (Variables|Default|SetisAttack true)
          (else
            (Animation|PlayAnimMontage "/Game/JWContent/Anim/Attack2_Montage.Attack2_Montage" 1.0 "None")
            (Variables|Default|SetisAttack true)))))))

(event Input|ActionEvents|InputActionRoll
  (params (Key :type Key%20Structure :default "None"))
  ;[1 1 1] 구르기 SpaceBar
  (:Pressed
    (if (not (Variables|Default|GetisAttack))
      (if (> (Math|Vector|VectorLength (Math|Vector|MakeVector (Input|AxisValues|GetMoveForward) (Input|AxisValues|GetMoveRight) 0.0)) 0.0)
        (Transformation|SetActorRotation (Pawn|GetControlRotation :!class /Script/Engine.Pawn)))
      (Animation|PlayAnimMontage "/Game/JWContent/Anim/Stand_To_Roll_Montage.Stand_To_Roll_Montage" 1.0 "None")
      (Variables|Default|SetisAttack true))))

(event Input|AxisEvents|InputAxisMoveForward
  (params (AxisValue :type Float%20%28single-precision%29))
  ;[1 1 1] 플레이어 이동
  (if (not (Variables|Default|GetisAttack))
    (Pawn|Input|AddMovementInput (Math|Vector|GetForwardVector (Math|Rotator|MakeRotator 0.0 0.0 (.Yaw (Math|Rotator|BreakRotator (Pawn|GetControlRotation :!class /Script/Engine.Pawn))))) AxisValue false)))

(event Input|AxisEvents|InputAxisMoveRight
  (params (AxisValue :type Float%20%28single-precision%29))
  ;[1 1 1] 플레이어 이동
  (if (not (Variables|Default|GetisAttack))
    (Pawn|Input|AddMovementInput (Math|Vector|GetRightVector (Math|Rotator|MakeRotator 0.0 0.0 (.Yaw (Math|Rotator|BreakRotator (Pawn|GetControlRotation :!class /Script/Engine.Pawn))))) AxisValue false)))

(event Input|AxisEvents|InputAxisTurn
  (params (AxisValue :type Float%20%28single-precision%29))
  (Pawn|Input|AddControllerYawInput AxisValue))

(event Input|AxisEvents|InputAxisLookUp
  (params (AxisValue :type Float%20%28single-precision%29))
  (Pawn|Input|AddControllerPitchInput AxisValue))

(event Input|KeyboardEvents|LeftShift
  (params (Key :type Key%20Structure :default "None"))
  ;[1 1 1] 특수 공격 Shift + Mouse Left
  (:Pressed
    (Variables|Default|SetSAttack true))
  (:Released
    (Variables|Default|SetSAttack false)))

(fn ConstructionScript)

(fn UseItemPotion)

(fn DamageUIEvent
  ;[1 1 1] 데미지 충격 표시
  (bind _returnvalue (UserInterface|CreateWidget "/Game/JWContent/Blueprint/BP_Damage.BP_Damage_C" (Game|GetPlayerController 0)))
  (UserInterface|Viewport|AddtoViewport _returnvalue 0)
  (Widget|RemovefromParent (Variables|Default|GetDamageUI)))